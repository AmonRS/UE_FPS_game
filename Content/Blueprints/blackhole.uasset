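; Blackhole actor that acts as a timed spawner, producing Targets actors at its own location.
; BeginPlay runs a latent loop that increments Targetcount, waits on a Delay of a few seconds, spawns one target, then wires back to the count check.
; The loop ends once Targetcount exceeds its hard-coded cap; Tick, overlap and the construction script are empty.
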(event EventBeginPlay
  (if (<= (Variables|Default|Gettargetcount) 200) :!label _label
    (Variables|Default|Settargetcount (+ (Variables|Default|Gettargetcount) 1))
    (Utilities|FlowControl|Delay 3.0)
    (Game|SpawnActorfromClass "/Game/Blueprints/targets.targets_C" (Math|Conversions|ToTransform(Vector) (Transformation|GetActorLocation self)) "Undefined" 0 0)
    (goto _label)))

(event Collision|EventActorBeginOverlap
  (params (OtherActor :type Actor%20Object%20Reference)))

(event EventTick
  (params (DeltaSeconds :type Float%20%28single-precision%29)))

(fn ConstructionScript)