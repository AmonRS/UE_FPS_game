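; A destructible target actor that takes a random color at spawn and is destroyed after being damaged.
; BeginPlay creates a dynamic instance of Target_mi on the Destructible component and randomizes its hue shift parameter.
; Any damage turns physics simulation off on that component, applies a radial impulse from the actor's location, then destroys the actor after a short delay.
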(event EventBeginPlay
  ;[1 1 1] random material at start
  (Rendering|Material|CreateDynamicMaterialInstance (Variables|Default|GetDestructible) 0 "/Game/materials/target_mi.target_mi" "None" :!class /Script/Engine.PrimitiveComponent)
  (Rendering|Material|SetScalarParameterValueonMaterials (Variables|Default|GetDestructible) "hueshiftpercentage" (Math|Random|RandomFloat)))

(event Collision|EventActorBeginOverlap
  (params (OtherActor :type Actor%20Object%20Reference)))

(event EventTick
  (params (DeltaSeconds :type Float%20%28single-precision%29)))

(event Game|Damage|EventAnyDamage
  (params (Damage :type Float%20%28single-precision%29) (DamageType :type Damage%20Type%20Object%20Reference) (InstigatedBy :type Controller%20Object%20Reference) (DamageCauser :type Actor%20Object%20Reference))
  (bind _destructible (Variables|Default|GetDestructible))
  ;[1 1 1] damage
  (Physics|SetSimulatePhysics _destructible false)
  (Physics|AddRadialImpulse _destructible (Transformation|GetActorLocation self) 5e+02 2e+03 "RIF_Constant" false)
  (Utilities|FlowControl|Delay 3.0)
  (Actor|DestroyActor))

(fn ConstructionScript)